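; BP_TestCharacter2 is a test character that switches its camera between attachment setups on number keys.
; Keys 1 and 3 reparent the camera to the spring arm or a Scene component, while key 2 passes no parent.
; A shared helper reattaches with world transform kept, then MoveComponentTo moves the camera, timed on key 2.
; The helper also adds an InterpToMovement component on every call, without configuring it.
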(event EventBeginPlay)

(event Collision|EventActorBeginOverlap
  (params (OtherActor :type Actor%20Object%20Reference)))

(event EventTick
  (params (DeltaSeconds :type Float%20%28single-precision%29)))

(event Input|KeyboardEvents|3
  (params (Key :type Key%20Structure))
  (bind _camera (Variables|Default|GetCamera))
  (:Pressed
    (CallFunction|NewFunction _camera (Variables|Default|GetScene))
    (Components|MoveComponentTo _camera "0, 0, 0" "0, 0, 0" false false 0.2 true)))

(event Input|KeyboardEvents|1
  (params (Key :type Key%20Structure))
  (bind _camera (Variables|Default|GetCamera))
  (:Pressed
    (CallFunction|NewFunction _camera (Variables|Default|GetSpringArm))
    (Components|MoveComponentTo _camera "0, 0, 0" "0, 0, 0" false false 0.2 true)))

(event Input|KeyboardEvents|2
  (params (Key :type Key%20Structure))
  (bind _camera (Variables|Default|GetCamera))
  (:Pressed
    (CallFunction|NewFunction _camera)
    (Components|MoveComponentTo _camera "0, 0, 0" "0, 0, 0" false false 3.0 false)))

(fn ConstructionScript)

(fn NewFunction
  (params (Target :type Camera%20Component%20Object%20Reference) (Parent :type Scene%20Component%20Object%20Reference))
  (Transformation|AttachComponentToComponent Target Parent "None" "KeepWorld" "KeepWorld" "KeepWorld" true)
  (AddComponent|AddInterptoMovementComponent))