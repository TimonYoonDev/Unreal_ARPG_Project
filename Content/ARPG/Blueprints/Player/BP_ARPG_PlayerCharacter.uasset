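; ARPG player character Blueprint that toggles weapon equip and unequip from the 1 key.
; A FlipFlop alternates between setting the WeaponEquip and WeaponUnEquip flags on the mesh's ABP_Manny animation instance.
; Each press starts a one-second InputTime lockout that Tick counts down.
; Once it expires, Tick clears both flags every frame, so they act as timed animation triggers.
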(event EventBeginPlay)

(event Collision|EventActorBeginOverlap
  (params (OtherActor :type Actor%20Object%20Reference)))

(event EventTick
  (params (DeltaSeconds :type Float%20%28single-precision%29))
  (if (> (Variables|Default|GetInputTime) 0.0)
    (Variables|Default|SetInputTime (- (Variables|Default|GetInputTime) DeltaSeconds))
    (else
      (bind _asabp_manny (Utilities|Casting|CastToABP_Manny (Components|SkeletalMesh|GetAnimInstance (Variables|Character|GetMesh))))
      (Variables|/Game/Characters/Mannequins/Animations/ABP_Manny.ABP_Manny_C|SetbWeaponEquip _asabp_manny false)
      (Variables|/Game/Characters/Mannequins/Animations/ABP_Manny.ABP_Manny_C|SetbWeaponUnEquip _asabp_manny false))))

(event Input|KeyboardEvents|1
  (params (Key :type Key%20Structure :default "None"))
  (bind _mesh (Variables|Character|GetMesh))
  (bind _returnvalue (Components|SkeletalMesh|GetAnimInstance _mesh))
  (:Pressed
    (if (not (> (Variables|Default|GetInputTime) 0.0))
      (Utilities|FlowControl|FlipFlop
        (:A
          (bind _asabp_manny (Utilities|Casting|CastToABP_Manny _returnvalue))
          (Variables|/Game/Characters/Mannequins/Animations/ABP_Manny.ABP_Manny_C|SetbWeaponEquip _asabp_manny true)
          (Variables|Default|SetInputTime 1.0))
        (:B
          (bind _asabp_manny_2 (Utilities|Casting|CastToABP_Manny _returnvalue))
          (Variables|/Game/Characters/Mannequins/Animations/ABP_Manny.ABP_Manny_C|SetbWeaponUnEquip _asabp_manny_2 true)
          (Variables|Default|SetInputTime 1.0))))))

(fn ConstructionScript)